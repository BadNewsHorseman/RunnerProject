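; Player character for an endless runner with flipbook sprites, auto-running along X with tap-to-jump and an optional double jump.
; Tick tracks distance, requests new ground from BP_MapSpawner, and drives flipbooks and gravity for snappier falls.
; Overlaps trigger pickups or traps that cost health and speed unless boosted.
; Falling, lost health or timer expiry flags the cause in BP_GameInstance, pauses and shows UMG_EndGame.
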(event OnComponentBeginOverlap(Box)
  (params (OverlappedComponent :type Primitive%20Component%20Object%20Reference) (OtherActor :type Actor%20Object%20Reference) (OtherComp :type Primitive%20Component%20Object%20Reference) (OtherBodyIndex :type Integer) (bFromSweep :type Boolean) (SweepResult :type Hit%20Result%20Structure%20%28by%20ref%29)))

(event OnComponentBeginOverlap(CapsuleComponent)
  (params (OverlappedComponent :type Primitive%20Component%20Object%20Reference) (OtherActor :type Actor%20Object%20Reference) (OtherComp :type Primitive%20Component%20Object%20Reference) (OtherBodyIndex :type Integer) (bFromSweep :type Boolean) (SweepResult :type Hit%20Result%20Structure%20%28by%20ref%29))
  (bind _charactermovement (Variables|Character|GetCharacterMovement))
  (bind _asbp_pickup_base (Utilities|Casting|CastToBP_Pickup_Base OtherActor)
    (:then
      (Default|Pickup _asbp_pickup_base))
    (:CastFailed
      (bind _asbp_trap_base (Utilities|Casting|CastToBP_Trap_Base OtherActor))
      (if (<= (- (Variables|Default|GetHealth) 1) 0)
        (Variables|/Game/Blueprints/Modes_Instances/BP_GameInstance.BP_GameInstance_C|SetHealth? (Variables|Default|GetGameInstanceRef) true)
        (Game|SetGamePaused true)
        (bind _returnvalue (UserInterface|CreateWidget "/Game/UMG/UMG_EndGame.UMG_EndGame_C"))
        (UserInterface|Viewport|AddtoViewport _returnvalue 0)
        (Actor|DestroyActor _asbp_trap_base)
        (elif (not (Variables|Default|GetBoostActive))
          (Variables|Default|SetHealth (- (Variables|Default|GetHealth) 1))
          (Variables|/Script/Engine.CharacterMovementComponent|SetMaxWalkSpeed _charactermovement 6e+02)
          (Utilities|FlowControl|RetriggerableDelay 0.5)
          (if (> (- (Variables|Default|GetCurrentMaxSpeed) 1e+02) 6e+02)
            (Variables|Default|SetCurrentMaxSpeed (- (Variables|Default|GetCurrentMaxSpeed) 1e+02))
            (else
              (Variables|Default|SetCurrentMaxSpeed 6e+02)))
          (Variables|/Script/Engine.CharacterMovementComponent|SetMaxWalkSpeed _charactermovement (Variables|Default|GetCurrentMaxSpeed))
          (Actor|DestroyActor _asbp_trap_base))))))

(event OnComponentBeginOverlap(Deleter)
  (params (OverlappedComponent :type Primitive%20Component%20Object%20Reference) (OtherActor :type Actor%20Object%20Reference) (OtherComp :type Primitive%20Component%20Object%20Reference) (OtherBodyIndex :type Integer) (bFromSweep :type Boolean) (SweepResult :type Hit%20Result%20Structure%20%28by%20ref%29)))

(event Custom|AddSpeed
  (params (AmtToAdd :type Integer))
  (bind _charactermovement (Variables|Character|GetCharacterMovement))
  (Variables|/Script/Engine.CharacterMovementComponent|SetMaxWalkSpeed _charactermovement (+ (Math|Conversions|ToFloat(Integer) AmtToAdd) (Variables|/Script/Engine.CharacterMovementComponent|GetMaxWalkSpeed _charactermovement))))

(event Custom|Timer
  (bind _output_get (Variables|Default|SetTimerRemaining (Utilities|Time|GetTimerRemainingTimebyHandle (Variables|Default|GetEndGameTimerHandle))))
  (Development|PrintString (Utilities|String|ToString(Integer) (Math|Float|Truncate _output_get)) true false "(R=0.000000,G=0.660000,B=1.000000,A=1.000000)" 0.49))

(event Custom|EndGame
  (Variables|/Game/Blueprints/Modes_Instances/BP_GameInstance.BP_GameInstance_C|SetTime? (Variables|Default|GetGameInstanceRef) true)
  (Game|SetGamePaused true)
  (bind _returnvalue (UserInterface|CreateWidget "/Game/UMG/UMG_EndGame.UMG_EndGame_C"))
  (UserInterface|Viewport|AddtoViewport _returnvalue 0))

(event Custom|StartGame
  (bind _returnvalue (Utilities|Time|SetTimerbyFunctionName 0 "EndGame" (Variables|Default|GetTimerRemaining)))
  (Variables|Default|SetEndGameTimerHandle _returnvalue)
  (Utilities|Time|SetTimerbyFunctionName 0 "Timer" 0.5 true)
  (Variables|Default|SetScaleValue 1.0))

(event Custom|AddHealth
  (Math|Integer|IncrementInt (Variables|Default|GetHealth)))

(event Custom|RetrySpeed
  (Variables|/Script/Engine.CharacterMovementComponent|SetMaxWalkSpeed (Variables|Character|GetCharacterMovement) 6e+02)
  (Utilities|FlowControl|RetriggerableDelay 2.0)
  (Variables|/Script/Engine.CharacterMovementComponent|SetMaxWalkSpeed (Variables|Character|GetCharacterMovement) (Variables|Default|GetCurrentMaxSpeed)))

(event EventBeginPlay
  (bind _outactors (Actor|GetAllActorsOfClass "/Game/Blueprints/MapSpawner/Other/BP_CheckPoint.BP_CheckPoint_C"))
  (Variables|Default|SetCurrentCheckpoint (Utilities|Array|Get(acopy) _outactors))
  (bind _asbp_game_instance (Utilities|Casting|CastToBP_GameInstance (Game|GetGameInstance)))
  (Variables|Default|SetGameInstanceRef _asbp_game_instance))

(event EventTick
  (params (DeltaSeconds :type Float%20%28single-precision%29))
  (bind _returnvalue (Transformation|GetActorLocation))
  (bind _returnvalue_2 (Transformation|GetActorLocation))
  (bind _sprite (Variables|Default|GetSprite))
  (bind _gameinstanceref (Variables|Default|GetGameInstanceRef))
  (bind _charactermovement (Variables|Character|GetCharacterMovement))
  (bind _spawnerref (Variables|Default|GetSpawnerRef))
  (bind (_x _y) (Math|Vector|BreakVector _returnvalue_2))
  (bind _spawnedgrounds (Variables|/Game/Blueprints/BP_MapSpawner.BP_MapSpawner_C|GetSpawnedGrounds _spawnerref))
  (Utilities|IsValid self
    (:Is%20Valid
      (if (== (Variables|Default|GetScaleValue) 1.0)
        (Utilities|FlowControl|Sequence
          (:then_0
            (Pawn|Input|AddMovementInput "1.000000, 0, 0" (Variables|Default|GetScaleValue) false)
            (bind _output_get (Variables|/Game/Blueprints/Modes_Instances/BP_GameInstance.BP_GameInstance_C|SetDistanceTravelled _gameinstanceref (Math|Float|Floor (/ (+ (Variables|Default|GetDistanceTravelled) (.X (Math|Vector|BreakVector (Transformation|GetActorLocation)))) 1e+02))))
            (if (> _output_get 0)
              (if (> _output_get (Variables|/Game/Blueprints/Modes_Instances/BP_GameInstance.BP_GameInstance_C|GetMaxDistanceTravelled _gameinstanceref))
                (Variables|/Game/Blueprints/Modes_Instances/BP_GameInstance.BP_GameInstance_C|SetMaxDistanceTravelled _gameinstanceref _output_get)))
            (if (< (.Z (Math|Vector|BreakVector _returnvalue)) -6e+02)
              (Variables|Default|SetScaleValue 0.0)
              (Transformation|SetActorLocation (Math|Vector|MakeVector (+ _x 1.5e+02) _y 6e+02) false false)
              (Variables|/Game/Blueprints/Modes_Instances/BP_GameInstance.BP_GameInstance_C|SetFall? (Variables|Default|GetGameInstanceRef) true)
              (Game|SetGamePaused true)
              (bind _returnvalue_3 (UserInterface|CreateWidget "/Game/UMG/UMG_EndGame.UMG_EndGame_C"))
              (UserInterface|Viewport|AddtoViewport _returnvalue_3 0)
              (elif (<= (Math|Vector|VectorLength (- (Transformation|GetActorLocation (Utilities|Array|Get(acopy) _spawnedgrounds (- (Utilities|Array|Length _spawnedgrounds) 1))) _returnvalue)) 1e+04)
                (Default|Spawn (Variables|Default|GetSpawnerRef)))))
          (:then_1
            (if (Variables|Default|GetJumped?)
              (Utilities|FlowControl|DoOnce false :!label _label
                (:Completed
                  (Sprite|SetFlipbook _sprite "/Game/Blueprints/Character/Sprites/Jump/FlipBook/Jump_FlipBook.Jump_FlipBook")
                  (Utilities|FlowControl|Delay 0.5)
                  (Sprite|SetFlipbook _sprite "/Game/Blueprints/Character/Sprites/Falling/FlipBook/Fall_FlipBook.Fall_FlipBook")
                  (Variables|/Script/Engine.CharacterMovementComponent|SetGravityScale _charactermovement 3e+01)))))
          (:then_2
            (if (AI|Components|NavMovement|IsFalling (Variables|Character|GetCharacterMovement))
              (if (not (Variables|Default|GetJumped?))
                (Sprite|SetFlipbook _sprite "/Game/Blueprints/Character/Sprites/Falling/FlipBook/Fall_FlipBook.Fall_FlipBook"))
              (else
                (Sprite|SetFlipbook _sprite "/Game/Blueprints/Character/Sprites/Run/FlipBooks/Run_FlipBook.Run_FlipBook")
                (Variables|Default|SetJumped? false)
                (Variables|Default|SetJumpable? true)
                (Variables|/Script/Engine.CharacterMovementComponent|SetGravityScale _charactermovement 5.0)
                (goto _label Reset))))
          (:then_3
            (Variables|Default|SetDistanceFromCheck (Math|Float|Truncate (/ (Math|Vector|VectorLength (- (Transformation|GetActorLocation (Variables|Default|GetCurrentCheckpoint)) (Transformation|GetActorLocation))) 1e+02)))))))))

(event Input|TouchEvents|InputTouch
  (params (Location :type Vector) (FingerIndex :type ETouchIndex%20Enum))
  (bind _charactermovement (Variables|Character|GetCharacterMovement))
  (:Pressed
    (if (Variables|Default|GetJumpable?)
      (if (and (Variables|Default|GetJumped?) (Variables|Default|GetDoubleJump?))
        (Character|LaunchCharacter "500.000000, 0,1500.000000" false false)
        (Variables|/Script/Engine.CharacterMovementComponent|SetGravityScale _charactermovement 1.0)
        (Variables|Default|SetJumpable? false)
        (Utilities|FlowControl|RetriggerableDelay 0.5)
        (Variables|/Script/Engine.CharacterMovementComponent|SetGravityScale _charactermovement 3e+01)
        (else
          (Character|Jump)
          (Variables|Default|SetJumped? true)))))
  (:Released
    (Utilities|FlowControl|Delay 0.5)
    (Variables|Default|SetJumped? false)))

(fn ConstructionScript
  (bind _outactors (Actor|GetAllActorsOfClass "/Game/Blueprints/BP_MapSpawner.BP_MapSpawner_C"))
  (Variables|Default|SetSpawnerRef (Utilities|Array|Get(acopy) _outactors)))