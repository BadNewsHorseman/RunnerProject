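; BP_CheckPoint is a self-replacing checkpoint that extends the player's game time and shows a growing bonus.
; On overlap, it spawns its successor ahead along X, passing on the raised bonus and a spawn distance that grows after the first few checkpoints.
; It updates the map spawner and character references, restarts the EndGame timer with added time, displays the bonus on the HUD, then destroys itself.
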(event OnComponentBeginOverlap(Box)
  (params (OverlappedComponent :type Primitive%20Component%20Object%20Reference) (OtherActor :type Actor%20Object%20Reference) (OtherComp :type Primitive%20Component%20Object%20Reference) (OtherBodyIndex :type Integer) (bFromSweep :type Boolean) (SweepResult :type Hit%20Result%20Structure%20%28by%20ref%29))
  (bind _mapspawnerref (Variables|Default|GetMapSpawnerRef))
  (bind _characterref (Variables|Default|GetCharacterRef))
  (bind _checkpoints (Variables|/Game/Blueprints/BP_MapSpawner.BP_MapSpawner_C|GetCheckPoints _mapspawnerref))
  (bind _asmy_character (Utilities|Casting|CastToMyCharacter OtherActor))
  (Utilities|IsValid self
    (:Is%20Valid
      (bind _result (Math|Integer|IncrementInt (Variables|/Game/Blueprints/Character/MyCharacter.MyCharacter_C|GetCheckpointsPassed _asmy_character))
        (:%20%20
          (if (<= _result 5)
            (Variables|Default|SetBonusToGive (+ (Variables|Default|GetBonusToGive) 500))
            (else
              (Utilities|FlowControl|DoOnce false
                (:Completed
                  (Variables|Default|SetBonusToGive (+ (Variables|Default|GetBonusToGive) 500))
                  (Variables|Default|SetNewDistanceToSpawn (+ (Variables|Default|GetNewDistanceToSpawn) 1e+04))))))
          (bind _returnvalue (Game|SpawnActorfromClass "BP_CheckPoint_C" (Math|Transform|MakeTransform (Math|Vector|MakeVector (+ (.X (Math|Vector|BreakVector (Transformation|GetActorLocation _asmy_character))) (Variables|Default|GetNewDistanceToSpawn)) 0.0 0.0) "0, 0, 0" "1,1,1") "Undefined" 0 (Variables|Default|GetNewDistanceToSpawn) (Variables|Default|GetBonusToGive) 0))
          (Utilities|Array|Add _checkpoints _returnvalue)
          (Utilities|Array|RemoveItem _checkpoints self)
          (Variables|/Game/Blueprints/Character/MyCharacter.MyCharacter_C|SetCurrentCheckpoint _characterref _returnvalue)
          (bind _output_get (Variables|/Game/Blueprints/Character/MyCharacter.MyCharacter_C|SetTimerRemaining _characterref (+ (Variables|/Game/Blueprints/Character/MyCharacter.MyCharacter_C|GetTimerRemaining _characterref) 2e+01)))
          (Variables|BP_CheckPoint_C|SetHUDRef _returnvalue (Variables|Default|GetHUDRef))
          (bind _returnvalue_2 (Utilities|Time|SetTimerbyFunctionName _characterref "EndGame" _output_get))
          (Variables|/Game/Blueprints/Character/MyCharacter.MyCharacter_C|SetEndGameTimerHandle _characterref _returnvalue_2)
          (Default|DisplayBonus (Variables|Default|GetHUDRef) (Variables|Default|GetBonusToGive))
          (Actor|DestroyActor))))))

(event EventBeginPlay
  (bind _outactors (Actor|GetAllActorsOfClass "/Game/Blueprints/BP_MapSpawner.BP_MapSpawner_C"))
  (Variables|Default|SetMapSpawnerRef (Utilities|Array|Get(acopy) _outactors))
  (bind _asmy_character (Utilities|Casting|CastToMyCharacter (Game|GetPlayerCharacter 0)))
  (Variables|Default|SetCharacterRef _asmy_character)
  (bind _foundwidgets (Widget|GetAllWidgetsOfClass "/Game/UMG/UMG_HUD.UMG_HUD_C" false))
  (Variables|Default|SetHUDRef (Utilities|Array|Get(acopy) _foundwidgets)))

(event Collision|EventActorBeginOverlap
  (params (OtherActor :type Actor%20Object%20Reference)))

(event EventTick
  (params (DeltaSeconds :type Float%20%28single-precision%29)))

(fn ConstructionScript)