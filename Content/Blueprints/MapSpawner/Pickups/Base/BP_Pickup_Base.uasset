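; Base pickup actor that grants the player gold, gems, speed or health according to its reward type, then destroys itself.
; BeginPlay caches the game instance for currency and the player character for stats.
; Speed past its cap or health past maximum instead rolls a consolation reward, usually gold and rarely a gem.
; Its sphere overlap event is empty, so nothing in this graph triggers the Pickup event.
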(event OnComponentBeginOverlap(Sphere)
  (params (OverlappedComponent :type Primitive%20Component%20Object%20Reference) (OtherActor :type Actor%20Object%20Reference) (OtherComp :type Primitive%20Component%20Object%20Reference) (OtherBodyIndex :type Integer) (bFromSweep :type Boolean) (SweepResult :type Hit%20Result%20Structure%20%28by%20ref%29)))

(event Custom|Pickup
  (bind _instanceref (Variables|Default|GetInstanceRef))
  (bind _instanceref_2 (Variables|Default|GetInstanceRef))
  (bind _rewardcount (Variables|Default|GetRewardCount))
  (bind _characterref (Variables|Default|GetCharacterRef))
  (bind _returnvalue (Math|Conversions|ToFloat(Integer) _rewardcount))
  (bind _charactermovement (Variables|/Script/Engine.Character|GetCharacterMovement _characterref))
  (bind _maxwalkspeed (Variables|/Script/Engine.CharacterMovementComponent|GetMaxWalkSpeed _charactermovement))
  (bind _returnvalue_2 (+ _maxwalkspeed _returnvalue))
  (switch Utilities|FlowControl|Switch|SwitchonE_RewardType (Variables|Default|GetRewardType)
    (:NewEnumerator0
      _)
    (:NewEnumerator1
      (Default|AddGold _instanceref _rewardcount))
    (:NewEnumerator2
      (Default|AddGems _instanceref _rewardcount))
    (:NewEnumerator3
      (if (Variables|/Game/Blueprints/Character/MyCharacter.MyCharacter_C|GetBoostActive _characterref)
        (Variables|/Game/Blueprints/Character/MyCharacter.MyCharacter_C|SetCurrentMaxSpeed _characterref _returnvalue_2)
        (else
          (Variables|/Game/Blueprints/Character/MyCharacter.MyCharacter_C|SetCurrentMaxSpeed _characterref _returnvalue_2)))
      (if (> _returnvalue_2 1.5e+03)
        (Variables|/Game/Blueprints/Character/MyCharacter.MyCharacter_C|SetCurrentMaxSpeed _characterref 1.5e+03)
        (if (<= (Math|Random|RandomIntegerinRange 0 100) 5) :!label _label
          (Default|AddGems _instanceref_2 1)
          (else
            (Default|AddGold _instanceref_2 25)))
        (else
          (Default|AddSpeed _characterref _rewardcount))))
    (:NewEnumerator4
      (if (> (+ (Variables|/Game/Blueprints/Character/MyCharacter.MyCharacter_C|GetHealth _characterref) 1) (Variables|/Game/Blueprints/Character/MyCharacter.MyCharacter_C|GetMaxHealth _characterref))
        (goto _label)
        (else
          (Default|AddHealth (Variables|Default|GetCharacterRef))))))
  (Actor|DestroyActor))

(event EventBeginPlay
  (bind _asbp_game_instance (Utilities|Casting|CastToBP_GameInstance (Game|GetGameInstance)))
  (Variables|Default|SetInstanceRef _asbp_game_instance)
  (bind _asmy_character (Utilities|Casting|CastToMyCharacter (Game|GetPlayerCharacter 0)))
  (Variables|Default|SetCharacterRef _asmy_character))

(fn ConstructionScript)