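; Map spawner that procedurally builds a chain of ground pieces for the theme selected in BP_GameMode.
; BeginPlay filters templates by theme name, then InitialSpawn places any "very"-named piece at the theme's first location and chains random templates end to end up to a length limit.
; Height is randomly high, middle or low, with Allow flags blocking direct high-to-low jumps.
; Spawn repeats that loop but is uncalled here; checkpoint spawning is unwired.
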(event EventBeginPlay
  (CallFunction|GetGroundTemplates)
  (CallFunction|InitialSpawn))

(event Collision|EventActorBeginOverlap
  (params (OtherActor :type Actor%20Object%20Reference)))

(event EventTick
  (params (DeltaSeconds :type Float%20%28single-precision%29)))

(fn ConstructionScript)

(fn InitialSpawn
  (bind _templatestouse (Variables|Default|GetTemplatesToUse))
  (bind _templatestouse_2 (Variables|Default|GetTemplatesToUse))
  (bind _templatestouse_3 (Variables|Default|GetTemplatesToUse))
  (for _array_element (Variables|Default|GetTemplatesToUse)
    (if (Utilities|String|Contains (Utilities|GetClassDisplayName _array_element) "very")
      (bind _returnvalue (Game|SpawnActorfromClass _array_element (Math|Transform|MakeTransform (.Value (Utilities|Map|Find (Variables|Default|GetFirstGroundLocation) (Variables|Default|GetThemeSelected))) "0, 0, 0" "1,1,1") "Undefined" 0 0))
      (Utilities|Array|Add (Variables|Default|GetSpawnedGrounds) _returnvalue)
      (Variables|Default|SetLastEndPointLocation (Transformation|GetWorldLocation (Variables|/Game/Blueprints/MapSpawner/Ground/Base/Ground_Template_Base.Ground_Template_Base_C|GetEndPoint _returnvalue)))
      (LocalVariables|SetLocalLengthSpawned (+ (LocalVariables|GetLocalLengthSpawned) (Math|Vector|VectorLength (- (Transformation|GetWorldLocation (Variables|/Game/Blueprints/MapSpawner/Ground/Base/Ground_Template_Base.Ground_Template_Base_C|GetEndPoint _returnvalue)) (Transformation|GetWorldLocation (Variables|/Game/Blueprints/MapSpawner/Ground/Base/Ground_Template_Base.Ground_Template_Base_C|GetStartPoint _returnvalue))))))))
  (while (< (LocalVariables|GetLocalLengthSpawned) 2e+04)
    (switch int (Math|Random|RandomIntegerinRange 0 2) :!label _label
      (:0
        (if (Variables|Default|GetAllowTop?)
          (bind _returnvalue_2 (Game|SpawnActorfromClass (Utilities|Array|Get(acopy) _templatestouse_3 (Math|Random|RandomIntegerinRange 0 (- (Utilities|Array|Length _templatestouse_3) 1))) (Math|Transform|MakeTransform (Math|Vector|MakeVector (.X (Math|Vector|BreakVector (Variables|Default|GetLastEndPointLocation))) (.Y (Math|Vector|BreakVector (Variables|Default|GetLastEndPointLocation))) 3e+02) "0, 0, 0" "1,1,1") "Undefined" 0 0))
          (Utilities|Array|Add (Variables|Default|GetSpawnedGrounds) _returnvalue_2)
          (Variables|Default|SetLastEndPointLocation (Transformation|GetWorldLocation (Variables|/Game/Blueprints/MapSpawner/Ground/Base/Ground_Template_Base.Ground_Template_Base_C|GetEndPoint _returnvalue_2)))
          (LocalVariables|SetLocalLengthSpawned (+ (LocalVariables|GetLocalLengthSpawned) (Math|Vector|VectorLength (- (Transformation|GetWorldLocation (Variables|/Game/Blueprints/MapSpawner/Ground/Base/Ground_Template_Base.Ground_Template_Base_C|GetEndPoint _returnvalue_2)) (Transformation|GetWorldLocation (Variables|/Game/Blueprints/MapSpawner/Ground/Base/Ground_Template_Base.Ground_Template_Base_C|GetStartPoint _returnvalue_2))))))
          (Variables|Default|SetAllowBottom? false)
          (Variables|Default|SetAllowMid? true)
          (Variables|Default|SetAllowTop? true)
          (else
            (goto _label))))
      (:1
        (if (Variables|Default|GetAllowMid?)
          (bind _returnvalue_3 (Game|SpawnActorfromClass (Utilities|Array|Get(acopy) _templatestouse (Math|Random|RandomIntegerinRange 0 (- (Utilities|Array|Length _templatestouse) 1))) (Math|Transform|MakeTransform (Math|Vector|MakeVector (.X (Math|Vector|BreakVector (Variables|Default|GetLastEndPointLocation))) (.Y (Math|Vector|BreakVector (Variables|Default|GetLastEndPointLocation))) 0.0) "0, 0, 0" "1,1,1") "Undefined" 0 0))
          (Utilities|Array|Add (Variables|Default|GetSpawnedGrounds) _returnvalue_3)
          (Variables|Default|SetLastEndPointLocation (Transformation|GetWorldLocation (Variables|/Game/Blueprints/MapSpawner/Ground/Base/Ground_Template_Base.Ground_Template_Base_C|GetEndPoint _returnvalue_3)))
          (LocalVariables|SetLocalLengthSpawned (+ (LocalVariables|GetLocalLengthSpawned) (Math|Vector|VectorLength (- (Transformation|GetWorldLocation (Variables|/Game/Blueprints/MapSpawner/Ground/Base/Ground_Template_Base.Ground_Template_Base_C|GetEndPoint _returnvalue_3)) (Transformation|GetWorldLocation (Variables|/Game/Blueprints/MapSpawner/Ground/Base/Ground_Template_Base.Ground_Template_Base_C|GetStartPoint _returnvalue_3))))))
          (Variables|Default|SetAllowBottom? true)
          (Variables|Default|SetAllowMid? true)
          (Variables|Default|SetAllowTop? true)
          (else
            (goto _label))))
      (:2
        (if (Variables|Default|GetAllowBottom?)
          (bind _returnvalue_4 (Game|SpawnActorfromClass (Utilities|Array|Get(acopy) _templatestouse_2 (Math|Random|RandomIntegerinRange 0 (- (Utilities|Array|Length _templatestouse_2) 1))) (Math|Transform|MakeTransform (Math|Vector|MakeVector (.X (Math|Vector|BreakVector (Variables|Default|GetLastEndPointLocation))) (.Y (Math|Vector|BreakVector (Variables|Default|GetLastEndPointLocation))) -3e+02) "0, 0, 0" "1,1,1") "Undefined" 0 0))
          (Utilities|Array|Add (Variables|Default|GetSpawnedGrounds) _returnvalue_4)
          (Variables|Default|SetLastEndPointLocation (Transformation|GetWorldLocation (Variables|/Game/Blueprints/MapSpawner/Ground/Base/Ground_Template_Base.Ground_Template_Base_C|GetEndPoint _returnvalue_4)))
          (LocalVariables|SetLocalLengthSpawned (+ (LocalVariables|GetLocalLengthSpawned) (Math|Vector|VectorLength (- (Transformation|GetWorldLocation (Variables|/Game/Blueprints/MapSpawner/Ground/Base/Ground_Template_Base.Ground_Template_Base_C|GetEndPoint _returnvalue_4)) (Transformation|GetWorldLocation (Variables|/Game/Blueprints/MapSpawner/Ground/Base/Ground_Template_Base.Ground_Template_Base_C|GetStartPoint _returnvalue_4))))))
          (Variables|Default|SetAllowBottom? true)
          (Variables|Default|SetAllowMid? true)
          (Variables|Default|SetAllowTop? false)
          (else
            (goto _label)))))))

(fn GetGroundTemplates
  (Utilities|Array|Clear (Variables|Default|GetTemplatesToUse))
  (bind _asbp_game_mode (Utilities|Casting|CastToBP_GameMode (Game|GetGameMode)))
  (Variables|Default|SetThemeSelected (Variables|/Game/Blueprints/Modes_Instances/BP_GameMode.BP_GameMode_C|GetThemeSelected _asbp_game_mode))
  (for _array_element (Variables|Default|GetTemplatesAvailable)
    (if (Utilities|String|Contains (Utilities|GetClassDisplayName _array_element) (Variables|Default|GetThemeSelected))
      (Utilities|Array|Add (Variables|Default|GetTemplatesToUse) _array_element))))

(fn Spawn
  (bind _templatestouse (Variables|Default|GetTemplatesToUse))
  (bind _templatestouse_2 (Variables|Default|GetTemplatesToUse))
  (bind _templatestouse_3 (Variables|Default|GetTemplatesToUse))
  (while (< (LocalVariables|GetLocalLengthSpawned) 2e+04)
    (switch int (Math|Random|RandomIntegerinRange 0 2) :!label _label
      (:0
        (if (Variables|Default|GetAllowTop?)
          (bind _returnvalue (Game|SpawnActorfromClass (Utilities|Array|Get(acopy) _templatestouse_3 (Math|Random|RandomIntegerinRange 0 (- (Utilities|Array|Length _templatestouse_3) 1))) (Math|Transform|MakeTransform (Math|Vector|MakeVector (.X (Math|Vector|BreakVector (Variables|Default|GetLastEndPointLocation))) (.Y (Math|Vector|BreakVector (Variables|Default|GetLastEndPointLocation))) 3e+02) "0, 0, 0" "1,1,1") "Undefined" 0 0))
          (Utilities|Array|Add (Variables|Default|GetSpawnedGrounds) _returnvalue)
          (Variables|Default|SetLastEndPointLocation (Transformation|GetWorldLocation (Variables|/Game/Blueprints/MapSpawner/Ground/Base/Ground_Template_Base.Ground_Template_Base_C|GetEndPoint _returnvalue)))
          (LocalVariables|SetLocalLengthSpawned (+ (LocalVariables|GetLocalLengthSpawned) (Math|Vector|VectorLength (- (Transformation|GetWorldLocation (Variables|/Game/Blueprints/MapSpawner/Ground/Base/Ground_Template_Base.Ground_Template_Base_C|GetEndPoint _returnvalue)) (Transformation|GetWorldLocation (Variables|/Game/Blueprints/MapSpawner/Ground/Base/Ground_Template_Base.Ground_Template_Base_C|GetStartPoint _returnvalue))))))
          (Variables|Default|SetAllowBottom? false)
          (Variables|Default|SetAllowMid? true)
          (Variables|Default|SetAllowTop? true)
          (else
            (goto _label))))
      (:1
        (if (Variables|Default|GetAllowMid?)
          (bind _returnvalue_2 (Game|SpawnActorfromClass (Utilities|Array|Get(acopy) _templatestouse (Math|Random|RandomIntegerinRange 0 (- (Utilities|Array|Length _templatestouse) 1))) (Math|Transform|MakeTransform (Math|Vector|MakeVector (.X (Math|Vector|BreakVector (Variables|Default|GetLastEndPointLocation))) (.Y (Math|Vector|BreakVector (Variables|Default|GetLastEndPointLocation))) 0.0) "0, 0, 0" "1,1,1") "Undefined" 0 0))
          (Utilities|Array|Add (Variables|Default|GetSpawnedGrounds) _returnvalue_2)
          (Variables|Default|SetLastEndPointLocation (Transformation|GetWorldLocation (Variables|/Game/Blueprints/MapSpawner/Ground/Base/Ground_Template_Base.Ground_Template_Base_C|GetEndPoint _returnvalue_2)))
          (LocalVariables|SetLocalLengthSpawned (+ (LocalVariables|GetLocalLengthSpawned) (Math|Vector|VectorLength (- (Transformation|GetWorldLocation (Variables|/Game/Blueprints/MapSpawner/Ground/Base/Ground_Template_Base.Ground_Template_Base_C|GetEndPoint _returnvalue_2)) (Transformation|GetWorldLocation (Variables|/Game/Blueprints/MapSpawner/Ground/Base/Ground_Template_Base.Ground_Template_Base_C|GetStartPoint _returnvalue_2))))))
          (Variables|Default|SetAllowBottom? true)
          (Variables|Default|SetAllowMid? true)
          (Variables|Default|SetAllowTop? true)
          (else
            (goto _label))))
      (:2
        (if (Variables|Default|GetAllowBottom?)
          (bind _returnvalue_3 (Game|SpawnActorfromClass (Utilities|Array|Get(acopy) _templatestouse_2 (Math|Random|RandomIntegerinRange 0 (- (Utilities|Array|Length _templatestouse_2) 1))) (Math|Transform|MakeTransform (Math|Vector|MakeVector (.X (Math|Vector|BreakVector (Variables|Default|GetLastEndPointLocation))) (.Y (Math|Vector|BreakVector (Variables|Default|GetLastEndPointLocation))) -3e+02) "0, 0, 0" "1,1,1") "Undefined" 0 0))
          (Utilities|Array|Add (Variables|Default|GetSpawnedGrounds) _returnvalue_3)
          (Variables|Default|SetLastEndPointLocation (Transformation|GetWorldLocation (Variables|/Game/Blueprints/MapSpawner/Ground/Base/Ground_Template_Base.Ground_Template_Base_C|GetEndPoint _returnvalue_3)))
          (LocalVariables|SetLocalLengthSpawned (+ (LocalVariables|GetLocalLengthSpawned) (Math|Vector|VectorLength (- (Transformation|GetWorldLocation (Variables|/Game/Blueprints/MapSpawner/Ground/Base/Ground_Template_Base.Ground_Template_Base_C|GetEndPoint _returnvalue_3)) (Transformation|GetWorldLocation (Variables|/Game/Blueprints/MapSpawner/Ground/Base/Ground_Template_Base.Ground_Template_Base_C|GetStartPoint _returnvalue_3))))))
          (Variables|Default|SetAllowBottom? true)
          (Variables|Default|SetAllowMid? true)
          (Variables|Default|SetAllowTop? false)
          (else
            (goto _label)))))))